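; Door actor that slides downward when the player activates a specific spaceship button.
; Each Tick it polls the player's BP_ThirdPersonCharacter for a LastActiveInteraction string matching that button, then overwrites it with "Activated" to consume the trigger.
; It then eases the root component down along Z with MoveComponentTo, printing debug strings; there is no closing logic.
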(event EventTick
  (params (DeltaSeconds :type Float%20%28single-precision%29))
  (bind _defaultsceneroot (Variables|Default|GetDefaultSceneRoot))
  (bind _returnvalue (Transformation|GetWorldLocation _defaultsceneroot))
  (bind _asbp_third_person_character (Utilities|Casting|CastToBP_ThirdPersonCharacter (Game|GetPlayerCharacter 0)))
  (if (Utilities|Enum|Equal(Enum) (Variables|/Game/ThirdPerson/Blueprints/BP_ThirdPersonCharacter.BP_ThirdPersonCharacter_C|GetLastActiveInteraction _asbp_third_person_character) "ButtonSpaceship1A")
    (Variables|/Game/ThirdPerson/Blueprints/BP_ThirdPersonCharacter.BP_ThirdPersonCharacter_C|SetLastActiveInteraction _asbp_third_person_character "Activated")
    (Development|PrintString "Door Animation")
    (Components|MoveComponentTo _defaultsceneroot (Math|Vector|MakeVector (.x _returnvalue) (.y _returnvalue) (- (.z _returnvalue) 6e+02)) (Transformation|GetWorldRotation _defaultsceneroot) false true 0.5 false)
    (Development|PrintString "Hello")))

(fn ConstructionScript)