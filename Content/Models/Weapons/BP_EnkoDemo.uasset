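; BP_EnkoDemo is a demo actor that shows off the glow material on a sword mesh.
; The construction script creates a dynamic material instance on the sword's first material slot.
; Overlapping the RandomColor component sets a random glow color, while overlapping OnOrOff alternately switches the glow on and off through a FlipFlop and a scalar parameter.
; Both triggers print a debug message.
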(event OnComponentBeginOverlap(Onoroff)
  (params (OverlappedComponent :type Primitive%20Component%20Object%20Reference) (OtherActor :type Actor%20Object%20Reference) (OtherComp :type Primitive%20Component%20Object%20Reference) (OtherBodyIndex :type Integer) (bFromSweep :type Boolean) (SweepResult :type Hit%20Result%20Structure%20%28by%20ref%29))
  (bind _dynamicswordmat (Variables|Default|GetDynamicSwordMat))
  (Utilities|FlowControl|FlipFlop
    (:A
      (Rendering|Material|SetScalarParameterValue _dynamicswordmat "ShouldNotGlow?" 0.0 :!class /Script/Engine.MaterialInstanceDynamic)
      (Development|PrintString "Glow on" true true "(R=0.108358,G=1.000000,B=0.000000,A=1.000000)"))
    (:B
      (Rendering|Material|SetScalarParameterValue _dynamicswordmat "ShouldNotGlow?" 1.0 :!class /Script/Engine.MaterialInstanceDynamic)
      (Development|PrintString "Glow Off" true true "(R=1.000000,G=0.029149,B=0.000000,A=1.000000)"))))

(event OnComponentBeginOverlap(RandomColor)
  (params (OverlappedComponent :type Primitive%20Component%20Object%20Reference) (OtherActor :type Actor%20Object%20Reference) (OtherComp :type Primitive%20Component%20Object%20Reference) (OtherBodyIndex :type Integer) (bFromSweep :type Boolean) (SweepResult :type Hit%20Result%20Structure%20%28by%20ref%29))
  (bind _output_get (Variables|Default|SetCurrentColor (Math|Color|MakeColor (Math|Random|RandomFloatinRange 0.0 1.0) (Math|Random|RandomFloatinRange 0.0 1.0) (Math|Random|RandomFloatinRange 0.0 1.0))))
  (Rendering|Material|SetVectorParameterValue (Variables|Default|GetDynamicSwordMat) "GlowColor" _output_get :!class /Script/Engine.MaterialInstanceDynamic)
  (Development|PrintString "ColorRandomized" true true _output_get))

(fn ConstructionScript
  (bind _returnvalue (Rendering|Material|CreateDynamicMaterialInstance (Variables|Default|GetSword) 0 0 "None" :!class /Script/Engine.PrimitiveComponent))
  (Variables|Default|SetDynamicSwordMat _returnvalue))