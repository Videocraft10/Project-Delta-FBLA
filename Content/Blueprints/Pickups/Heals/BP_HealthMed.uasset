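; BP_HealthMed is a medium health pickup actor that bobs in place and disappears when touched; it applies no healing itself.
; A timeline started on BeginPlay drives the mesh's vertical bounce, alongside a dynamic material instance created for the glow.
; The first sphere overlap by anything runs a one-shot glow timeline on that material.
; When it finishes, the mesh hides, sparkles stop, and the actor destroys itself after a short delay.
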(event OnComponentBeginOverlap(Sphere)
  (params (OverlappedComponent :type Primitive%20Component%20Object%20Reference) (OtherActor :type Actor%20Object%20Reference) (OtherComp :type Primitive%20Component%20Object%20Reference) (OtherBodyIndex :type Integer) (bFromSweep :type Boolean) (SweepResult :type Hit%20Result%20Structure%20%28by%20ref%29))
  (Development|PrintString "MedOverlap")
  (Utilities|FlowControl|DoOnce false
    (:Completed
      (bind _glow (Timeline|StartGlow Play)
        (:Update
          (Rendering|Material|SetScalarParameterValue (stale EventBeginPlay _returnvalue) "GlowIntensity" _glow :!class /Script/Engine.MaterialInstanceDynamic))
        (:Finished
          (Development|PrintString "MedGlow")
          (Rendering|SetVisibility (Variables|Default|GetHealthMedMesh) false false)
          (Effects|Components|ParticleSystem|SetEmitterEnable (Variables|Default|GetSparkles) "HealthMedSparkles" false)
          (Utilities|FlowControl|Delay 2.0)
          (Actor|DestroyActor))))))

(event Collision|EventActorBeginOverlap
  (params (OtherActor :type Actor%20Object%20Reference)))

(event EventTick
  (params (DeltaSeconds :type Float%20%28single-precision%29)))

(event EventBeginPlay
  (bind _returnvalue (Rendering|Material|CreateDynamicMaterialInstance (Variables|Default|GetHealthMedMesh) 0 "/Game/Models/Pickups/Health/Med/MI_HealthPackMedTex.MI_HealthPackMedTex" "None" :!class /Script/Engine.PrimitiveComponent))
  (bind _sine (Timeline|HealthBounce Play)
    (:Update
      (Transformation|SetRelativeLocation (Variables|Default|GetHealthMedMesh) (Math|Vector|MakeVector 0.0 0.0 _sine) false false))))

(fn ConstructionScript)