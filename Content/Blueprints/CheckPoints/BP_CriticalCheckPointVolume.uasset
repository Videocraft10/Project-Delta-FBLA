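; BP_CriticalCheckPointVolume is a trigger volume that registers itself as the player's latest critical checkpoint.
; When an ALS_AnimMan_CharacterBP begins overlapping the actor or stops overlapping its CollisionComponent, it sets LastCritCheckpoint on ALS_GameMode_SP to itself.
; Both paths share a Triggerd flag, so the checkpoint registers only once, and print debug strings on saving.
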(event OnComponentEndOverlap(CollisionComponent)
  (params (OverlappedComponent :type Primitive%20Component%20Object%20Reference) (OtherActor :type Actor%20Object%20Reference) (OtherComp :type Primitive%20Component%20Object%20Reference) (OtherBodyIndex :type Integer))
  (if (not (Variables|Default|GetTriggerd))
    (Utilities|Casting|CastToALS_AnimMan_CharacterBP OtherActor)
    (bind _asals_game_mode_sp (Utilities|Casting|CastToALS_GameMode_SP (Game|GetGameMode)))
    (Variables|/Game/AdvancedLocomotionV4/Blueprints/GameModes/ALS_GameMode_SP.ALS_GameMode_SP_C|SetLastCritCheckpoint _asals_game_mode_sp self)
    (Development|PrintString "CritCheckpoint" true true "(R=0.000000,G=1.000000,B=0.666948,A=1.000000)")
    (Variables|Default|SetTriggerd true)
    (Development|PrintString "Saved")))

(event EventBeginPlay)

(event Collision|EventActorBeginOverlap
  (params (OtherActor :type Actor%20Object%20Reference))
  (if (not (Variables|Default|GetTriggerd))
    (Utilities|Casting|CastToALS_AnimMan_CharacterBP OtherActor)
    (bind _asals_game_mode_sp (Utilities|Casting|CastToALS_GameMode_SP (Game|GetGameMode)))
    (Variables|/Game/AdvancedLocomotionV4/Blueprints/GameModes/ALS_GameMode_SP.ALS_GameMode_SP_C|SetLastCritCheckpoint _asals_game_mode_sp self)
    (Development|PrintString "CritCheckpoint" true true "(R=0.000000,G=1.000000,B=0.666948,A=1.000000)")
    (Variables|Default|SetTriggerd true)
    (Development|PrintString "Saved")))

(event EventTick
  (params (DeltaSeconds :type Float%20%28single-precision%29)))

(fn ConstructionScript)