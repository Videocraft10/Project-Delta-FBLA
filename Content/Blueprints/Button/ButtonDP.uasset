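; ButtonDP is an interactable button that offers an interaction while its Box trigger is overlapped.
; On begin overlap it creates a WB_Interact prompt, fades it in, then marks the player's BP_DeltaMovmentSys interaction valid as "ButtonSpaceship1".
; On end overlap it reverses the fade, clears that valid flag and removes the widget after a short delay.
; Neither overlap event checks which actor triggered it.
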(event OnComponentBeginOverlap(Box)
  (params (OverlappedComponent :type Primitive%20Component%20Object%20Reference) (OtherActor :type Actor%20Object%20Reference) (OtherComp :type Primitive%20Component%20Object%20Reference) (OtherBodyIndex :type Integer) (bFromSweep :type Boolean) (SweepResult :type Hit%20Result%20Structure%20%28by%20ref%29))
  (Development|PrintString "ButtonOverlap")
  (bind _returnvalue (UserInterface|CreateWidget "/Game/Widgets/PlayerUI/WB_Interact.WB_Interact_C"))
  (UserInterface|Viewport|AddtoViewport _returnvalue 0)
  (UserInterface|Animation|PlayAnimation _returnvalue (Variables|/Game/Widgets/PlayerUI/WB_Interact.WB_Interact_C|GetTextFadeIn _returnvalue) 0.0 1 "Forward" 1.0 false)
  (bind _asbp_delta_movment_sys (Utilities|Casting|CastToBP_DeltaMovmentSys (Game|GetPlayerCharacter 0)))
  (Variables|/Game/Blueprints/CharacterClasses/BP_DeltaMovmentSys.BP_DeltaMovmentSys_C|SetLast%20Active%20Interaction _asbp_delta_movment_sys "ButtonSpaceship1")
  (Variables|/Game/Blueprints/CharacterClasses/BP_DeltaMovmentSys.BP_DeltaMovmentSys_C|SetValid%20Interaction? _asbp_delta_movment_sys true))

(event OnComponentEndOverlap(Box)
  (params (OverlappedComponent :type Primitive%20Component%20Object%20Reference) (OtherActor :type Actor%20Object%20Reference) (OtherComp :type Primitive%20Component%20Object%20Reference) (OtherBodyIndex :type Integer))
  (UserInterface|Animation|PlayAnimation (stale OnComponentBeginOverlap(Box) _returnvalue) (Variables|/Game/Widgets/PlayerUI/WB_Interact.WB_Interact_C|GetTextFadeIn (stale OnComponentBeginOverlap(Box) _returnvalue)) 0.0 1 "Reverse" 1.0 false)
  (Variables|/Game/Blueprints/CharacterClasses/BP_DeltaMovmentSys.BP_DeltaMovmentSys_C|SetValid%20Interaction? (stale OnComponentBeginOverlap(Box) _asbp_delta_movment_sys) false)
  (Development|PrintString "Unoverlaped")
  (Utilities|FlowControl|Delay 0.25)
  (Widget|RemovefromParent (stale OnComponentBeginOverlap(Box) _returnvalue)))

(fn ConstructionScript)